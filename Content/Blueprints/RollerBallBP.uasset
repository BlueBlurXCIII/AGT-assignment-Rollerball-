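; RollerBallBP is the roller ball Blueprint that tracks elapsed time and score as it touches pickups.
; BeginPlay creates and stores the PlayerHUD widget and adds it to the viewport, while Tick accumulates delta time into a seconds counter.
; Overlaps run a Sequence of casts for four pickup classes, each playing the same sound and adding a tier-specific amount to the points total.
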(event EventActorBeginOverlap
  (params (OtherActor :type Actor%20Object%20Reference))
  (Utilities|FlowControl|Sequence
    (:then_0
      ;[1 1 1] Handle points (small)
      (Utilities|Casting|CastToPickup OtherActor)
      (Audio|PlaySoundatLocation "/Game/Audio/146727__fins__energy.146727__fins__energy" (Transformation|GetActorLocation))
      (Variables|Default|SetP_Points (+ (Variables|Default|GetP_Points) 100)))
    (:then_1
      ;[1 1 1] Handle points (med)
      (Utilities|Casting|CastToPickupMed OtherActor)
      (Audio|PlaySoundatLocation "/Game/Audio/146727__fins__energy.146727__fins__energy" (Transformation|GetActorLocation))
      (Variables|Default|SetP_Points (+ (Variables|Default|GetP_Points) 300)))
    (:then_2
      ;[1 1 1] Handle points (large)
      (Utilities|Casting|CastToPickupLarge OtherActor)
      (Audio|PlaySoundatLocation "/Game/Audio/146727__fins__energy.146727__fins__energy" (Transformation|GetActorLocation))
      (Variables|Default|SetP_Points (+ (Variables|Default|GetP_Points) 1000)))
    (:then_3
      ;[1 1 1] Handle points (mega)
      (Utilities|Casting|CastToMegaSphere OtherActor)
      (Audio|PlaySoundatLocation "/Game/Audio/146727__fins__energy.146727__fins__energy" (Transformation|GetActorLocation))
      (Variables|Default|SetP_Points (+ (Variables|Default|GetP_Points) 10000)))))

(event EventTick
  (params (DeltaSeconds :type Float%20%28single-precision%29))
  ;[1 1 1] Stopwatch timer
  (Variables|Default|SetSeconds (+ DeltaSeconds (Variables|Default|GetSeconds))))

(event EventBeginPlay
  ;[1 1 1] Init HUD
  (bind _returnvalue (UserInterface|CreateWidget "/Game/Blueprints/PlayerHUD.PlayerHUD_C"))
  (Variables|Default|SetGameHUDWidget _returnvalue)
  (UserInterface|Viewport|AddtoViewport (Variables|Default|GetGameHUDWidget)))

(fn ConstructionScript)